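; BP_Trigger is an overlap trigger that toggles a point light, gated behind the player's keys.
; BeginPlay stores the light's intensity, turns it off and caches the BP_ThirdPersonCharacter.
; On first overlap by a "Player"-tagged actor with HasKeys, the keys move into the socket; a FlipFlop then switches the light between saved intensity and zero on that and every later overlap.
; An alternative intensity-check toggle is left unconnected.
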(event EventBeginPlay
  (bind _pointlight (Variables|Default|GetPointLight))
  ;[0.15 0.15 0.15 0.5] Save current light intensity in variable
  (Variables|Default|SetLightIntensity (Variables|/Script/Engine.LightComponentBase|GetIntensity _pointlight))
  (Rendering|Components|Light|SetIntensity _pointlight 0.0)
  ;[0.15 0.15 0.15 0.5] Save the player instance
  (bind _asbp_third_person_character (Utilities|Casting|CastToBP_ThirdPersonCharacter (Game|GetPlayerCharacter 0))
    (:then
      (Variables|Default|SetPlayer _asbp_third_person_character))
    (:CastFailed
      (Development|PrintString "Not using the correct character!" true true "(R=1.000000,G=0.000000,B=0.183850,A=1.000000)"))))

(event Collision|EventActorBeginOverlap
  (params (OtherActor :type Actor%20Object%20Reference))
  (bind _player (Variables|Default|GetPlayer))
  (if (Actor|ActorHasTag OtherActor "Player")
    (if (Variables|Default|GetHasKeysInSocket)
      (Development|PrintString "Player : Flip flop Portal" true true "(R=1.000000,G=0.000000,B=0.105512,A=1.000000)" :!label _label)
      (bind _isa (Utilities|FlowControl|FlipFlop)
        (:A
          _)
        (:B
          _))
      (Rendering|Components|Light|SetIntensity (Variables|Default|GetPointLight) (Math|Float|SelectFloat (Variables|Default|GetLightIntensity) 0.0 _isa))
      (elif (Variables|/Game/BluePrintsClasses/Character/BP_ThirdPersonCharacter.BP_ThirdPersonCharacter_C|GetHas%20Keys _player)
        (Variables|/Game/BluePrintsClasses/Character/BP_ThirdPersonCharacter.BP_ThirdPersonCharacter_C|SetHas%20Keys _player false)
        (Variables|Default|SetHasKeysInSocket true)
        (goto _label)
        (else
          (Development|PrintString "No keys or not all"))))))

(fn ConstructionScript)