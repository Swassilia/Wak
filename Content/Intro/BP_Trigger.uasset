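; BP_Trigger is a trigger actor with a battery-powered point light that the player switches by overlapping it.
; BeginPlay stores the light's intensity, turns it off and caches the BP_FirstPersonCharacter player.
; An overlap by a "Player"-tagged actor moves the player's battery into the socket if it is empty, or prints "No battery".
; Once powered, each overlap flip-flops the intensity between the saved value and zero.
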(event EventBeginPlay
  (bind _pointlight (Variables|Default|GetPointLight))
  ;[0.15 0.15 0.15 0.5] Save current light intensity in variable
  (Variables|Default|SetLightIntensity (Variables|/Script/Engine.LightComponentBase|GetIntensity _pointlight))
  (Rendering|Components|Light|SetIntensity _pointlight 0.0)
  ;[0.15 0.15 0.15 0.5] Save the player instance
  (bind _asbp_first_person_character (Utilities|Casting|CastToBP_FirstPersonCharacter (Game|GetPlayerCharacter 0))
    (:then
      (Variables|Default|SetPlayer _asbp_first_person_character))
    (:CastFailed
      (Development|PrintString "Not using the correct character!" true true "(R=1.000000,G=0.000000,B=0.183850,A=1.000000)"))))

(event Collision|EventActorBeginOverlap
  (params (OtherActor :type Actor%20Object%20Reference))
  (if (Actor|ActorHasTag OtherActor "Player")
    (if (Variables|Default|GetHasBatteryInSocket)
      (Development|PrintString "Player : Flip flop light" true true "(R=1.000000,G=0.000000,B=0.105512,A=1.000000)" :!label _label)
      (bind _isa (Utilities|FlowControl|FlipFlop)
        (:A
          _)
        (:B
          _))
      (Rendering|Components|Light|SetIntensity (Variables|Default|GetPointLight) (Math|Float|SelectFloat (Variables|Default|GetLightIntensity) 0.0 _isa))
      (elif (Variables|/Game/FirstPerson/Blueprints/BP_FirstPersonCharacter.BP_FirstPersonCharacter_C|GetHasBattery (Variables|Default|GetPlayer))
        (Variables|/Game/FirstPerson/Blueprints/BP_FirstPersonCharacter.BP_FirstPersonCharacter_C|SetHasBattery (Variables|Default|GetPlayer) false)
        (Variables|Default|SetHasBatteryInSocket true)
        (goto _label)
        (else
          (Development|PrintString "No battery"))))))

(fn ConstructionScript)